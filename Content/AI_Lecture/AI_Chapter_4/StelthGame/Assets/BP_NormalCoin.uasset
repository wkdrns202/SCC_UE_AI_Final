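; BP_NormalCoin is a coin actor that bobs in place and destroys itself when any actor overlaps it.
; On BeginPlay it stores its start location and calls Pump, which plays a timeline that lerps the actor between that location and a point slightly above it.
; The timeline's Finished pin calls Pump again, so the motion repeats without Tick.
; The overlap handler has no actor filter and awards no score.
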(event Custom|Pump
  (bind _initcoinlocation (Variables|Default|GetInitCoinLocation))
  (bind _newtrack_0 (Timeline|Timeline_0 PlayFromStart)
    (:Update
      (Transformation|SetActorLocation (Math|Vector|Lerp(Vector) (Variables|Default|GetInitCoinLocation) (Math|Vector|MakeVector (.x _initcoinlocation) (.y _initcoinlocation) (+ (.z _initcoinlocation) 5e+01)) _newtrack_0) false false))
    (:Finished
      (CallFunction|Pump))))

(event EventBeginPlay
  (Variables|Default|SetInitCoinLocation (Transformation|GetActorLocation))
  (CallFunction|Pump))

(event Collision|EventActorBeginOverlap
  (params (OtherActor :type Actor%20Object%20Reference))
  (Actor|DestroyActor))

(event EventTick
  (params (DeltaSeconds :type Float%20%28single-precision%29)))

(fn ConstructionScript)