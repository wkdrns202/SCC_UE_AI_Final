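; BP_SurvailanceCamera is a surveillance camera actor for a stealth game that continuously sweeps its yaw.
; BeginPlay caches the starting rotation, then calls the Surveilance event.
; A Timeline track drives a lerp between that rotation and a fixed yaw offset, and Surveilance restarts the Timeline whenever it finishes.
; The graph handles rotation only, with no detection logic.
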(event Custom|Surveilance
  (bind _init_rotation (Variables|Default|GetInit_Rotation))
  (bind _newtrack_0 (Timeline|Timeline PlayFromStart)
    (:Update
      (Transformation|SetActorRotation (Math|Rotator|Lerp(Rotator) (Variables|Default|GetInit_Rotation) (Math|Rotator|MakeRotator (.roll _init_rotation) (.pitch _init_rotation) (- (.yaw _init_rotation) 5e+01)) _newtrack_0)))
    (:Finished
      (CallFunction|Surveilance))))

(event EventBeginPlay
  (Variables|Default|SetInit_Rotation (Transformation|GetActorRotation))
  (CallFunction|Surveilance))

(event Collision|EventActorBeginOverlap
  (params (OtherActor :type Actor%20Object%20Reference)))

(event EventTick
  (params (DeltaSeconds :type Float%20%28single-precision%29)))

(fn ConstructionScript)