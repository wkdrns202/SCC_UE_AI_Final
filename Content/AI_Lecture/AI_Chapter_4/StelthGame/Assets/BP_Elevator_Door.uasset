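; Elevator door actor for the stealth game that swings open on trigger overlaps, gated by second-floor coins from the front.
; An FW_Box overlap counts BP_Coins flagged IsOn2F and calls Activate, which rotates the door by Timeline only if none remain and FloorMoving is false.
; That Timeline sets FloorMoving from the door's angle, while BW_Box opens it wider without checks for 1F-to-2F travel.
; DoOnce nodes block retriggering until each Timeline finishes.
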(event OnComponentBeginOverlap(FW_Box)
  (params (OverlappedComponent :type Primitive%20Component%20Object%20Reference) (OtherActor :type Actor%20Object%20Reference) (OtherComp :type Primitive%20Component%20Object%20Reference) (OtherBodyIndex :type Integer) (bFromSweep :type Boolean) (SweepResult :type Hit%20Result%20Structure%20%28by%20ref%29))
  ;[0.15 0.15 0.15 0.5] 엘레베이터 작동 검증 및 Trigger 로직
  (Variables|Default|Set2FCoins 0)
  (bind _outactors (Actor|GetAllActorsOfClass "/Game/AILecture/AILecture_4/Coin/BP_Coin.BP_Coin_C"))
  (for _array_element _outactors
    (bind _output_get (Variables|Default|SetArray%20Element _array_element))
    (if (Variables|/Script/SCC_UEAI_Lecture.Item_Coin|GetbIsOn2F _output_get)
      (Math|Integer|IncrementInt (Variables|Default|Get2FCoins))))
  (CallFunction|Activate))

(event OnComponentBeginOverlap(BW_Box)
  (params (OverlappedComponent :type Primitive%20Component%20Object%20Reference) (OtherActor :type Actor%20Object%20Reference) (OtherComp :type Primitive%20Component%20Object%20Reference) (OtherBodyIndex :type Integer) (bFromSweep :type Boolean) (SweepResult :type Hit%20Result%20Structure%20%28by%20ref%29))
  ;[0.15 0.15 0.15 0.5] 1층->2층 이동시 개문
  (Utilities|FlowControl|DoOnce false :!label _label
    (:Completed
      (bind _newtrack_0 (Timeline|Timeline_0 Play)
        (:Update
          (Transformation|SetRelativeRotation (Variables|Default|GetDoor) (Math|Rotator|MakeRotator 0.0 0.0 (Math|Float|Lerp 0.0 -115.0 _newtrack_0)) false false))
        (:Finished
          (goto _label Reset))))))

(event Custom|Activate
  ;[0.15 0.15 0.15 0.5] 엘레베이터 작동 로직
  (if (not (Math|Conversions|ToBoolean(Integer) (Variables|Default|Get2FCoins)))
    (if (not (Variables|Default|GetFloorMoving?))
      (Utilities|FlowControl|DoOnce false :!label _label
        (:Completed
          (bind _newtrack_0 (Timeline|Timeline Play)
            (:Update
              (Transformation|SetRelativeRotation (Variables|Default|GetDoor) (Math|Rotator|MakeRotator 0.0 0.0 (Math|Float|Lerp 0.0 -9e+01 _newtrack_0)) false false)
              (if (< (Math|Float|Lerp 0.0 -9e+01 _newtrack_0) -15.0)
                (Variables|Default|SetFloorMoving? true)
                (else
                  (Variables|Default|SetFloorMoving? false))))
            (:Finished
              (goto _label Reset))))))))

(event EventBeginPlay)

(event Collision|EventActorBeginOverlap
  (params (OtherActor :type Actor%20Object%20Reference)))

(event EventTick
  (params (DeltaSeconds :type Float%20%28single-precision%29)))

(fn ConstructionScript)