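; BP_Elevator_floor is an elevator floor actor that travels vertically when triggered.
; Overlapping its Box while the floor is near ground height sets FloorMoving on a Target reference and starts the move.
; Tick also polls that flag, so setting it elsewhere can start the move through a DoOnce.
; A Timeline lerps Z between fixed world heights at the starting XY, then clears the flag and resets the DoOnce.
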(event OnComponentBeginOverlap(Box)
  (params (OverlappedComponent :type Primitive%20Component%20Object%20Reference) (OtherActor :type Actor%20Object%20Reference) (OtherComp :type Primitive%20Component%20Object%20Reference) (OtherBodyIndex :type Integer) (bFromSweep :type Boolean) (SweepResult :type Hit%20Result%20Structure%20%28by%20ref%29))
  (if (< (.z (Transformation|GetActorLocation)) 5)
    (Variables|/Game/AI_Lecture/AI_Chapter_4/StelthGame/Assets/BP_Elevator_Door.BP_Elevator_Door_C|SetFloorMoving? (Variables|Default|GetTarget) true)
    (CallFunction|Move)))

(event Custom|Move
  (bind _initlocation (Variables|Default|GetInitLocation))
  ;[0.15 0.15 0.15 0.5] 승강기 활성화
  (bind _newtrack_0 (Timeline|Timeline PlayFromStart)
    (:Update
      (Transformation|SetActorLocation (Math|Vector|MakeVector (.x _initlocation) (.y _initlocation) (Math|Float|Lerp 0.06 428.0 _newtrack_0)) false false))
    (:Finished
      (Variables|/Game/AI_Lecture/AI_Chapter_4/StelthGame/Assets/BP_Elevator_Door.BP_Elevator_Door_C|SetFloorMoving? (Variables|Default|GetTarget) false)
      (Utilities|FlowControl|DoOnce false) ; enters at Reset
    )))

(event EventBeginPlay
  (Variables|Default|SetInitLocation (Transformation|GetActorLocation)))

(event Collision|EventActorBeginOverlap
  (params (OtherActor :type Actor%20Object%20Reference)))

(event EventTick
  (params (DeltaSeconds :type Float%20%28single-precision%29))
  (if (Variables|/Game/AI_Lecture/AI_Chapter_4/StelthGame/Assets/BP_Elevator_Door.BP_Elevator_Door_C|GetFloorMoving? (Variables|Default|GetTarget))
    (Utilities|FlowControl|DoOnce false
      (:Completed
        (CallFunction|Move)))))

(fn ConstructionScript)